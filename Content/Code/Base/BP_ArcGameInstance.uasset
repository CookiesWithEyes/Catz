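; Arc game instance Blueprint with a stubbed hook for applying "Neco" settings; both its event and its settings function are empty.
; Disconnected nodes would split a "///"-delimited string into X, Y and SoundLevel, debug-printing each piece, though the source string is blank.
; Further unwired nodes would set a base sound mix and override Master sound class volume from SoundLevel scaled down by ten.
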(event `ApplydotNecoSettings`)

(fn `SetSettingsFromNeco`)